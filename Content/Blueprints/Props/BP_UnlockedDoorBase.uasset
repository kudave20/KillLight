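; Base Blueprint for an unlocked door prop that swings open and shut when interacted with.
; Each interact toggles a flag that plays or reverses a timeline, which lerps the Door component's relative yaw through a quarter turn.
; A CompletelyClosed flag limits the open sound to starts from fully shut, while the close sound plays when the reverse finishes.
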(event EventOnInteract
  (bind _output_get (Variables|Default|SetbClosed (not (Variables|Default|GetbClosed))))
  (if _output_get
    (if (Variables|Default|GetbCompletelyClosed)
      (Variables|Default|SetbCompletelyClosed false)
      (Audio|PlaySoundatLocation "/Game/Sounds/DoorOpenSound_Cue.DoorOpenSound_Cue" (Transformation|GetActorLocation) "0, 0, 0" 1.0 1.0 0.0 0 0 0 0)
      (bind (_direction _doortrack) (Timeline|OpenDoorTimeline Play)
        (:Update
          (Transformation|SetRelativeRotation (Variables|Default|GetDoor) (Math|Rotator|MakeRotator 0.0 0.0 (Math|Float|Lerp 0.0 9e+01 _doortrack)) false false))
        (:Finished
          (switch Utilities|FlowControl|Switch|SwitchonETimelineDirection _direction
            (:Backward
              (Audio|PlaySoundatLocation "/Game/Sounds/DoorCloseSound_Cue.DoorCloseSound_Cue" (Transformation|GetActorLocation) "0, 0, 0" 1.0 1.0 0.0 0 0 0 0)
              (Variables|Default|SetbCompletelyClosed true)))))
      (else
        (Timeline|OpenDoorTimeline Play)))
    (else
      (Timeline|OpenDoorTimeline Reverse))))

(fn ConstructionScript)