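; BP_UnlockedDoor_01 is an interactable door prop that toggles open or closed each time OnInteract fires.
; Interaction flips an Open flag, plays the matching open or close sound at the actor's location, and runs a timeline forward or in reverse.
; The timeline's float lerps the Door component's relative yaw to swing it a quarter turn, always restarting from either end rather than the current position.
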(event EventOnInteract
  (bind _returnvalue (Transformation|GetActorLocation))
  (bind _output_get (Variables|Default|SetbOpen (not (Variables|Default|GetbOpen))))
  (if _output_get
    (Audio|PlaySoundatLocation "/Game/Sounds/DoorOpenSound_Cue.DoorOpenSound_Cue" _returnvalue "0, 0, 0" 1.0 1.0 0.0 0 0 0 0)
    (bind _doorfloat (Timeline|OpenDoorTimeline PlayFromStart)
      (:Update
        (Transformation|SetRelativeRotation (Variables|Default|GetDoor) (Math|Rotator|MakeRotator 0.0 0.0 (Math|Float|Lerp 0.0 9e+01 _doorfloat)) false false)))
    (else
      (Audio|PlaySoundatLocation "/Game/Sounds/DoorCloseSound_Cue.DoorCloseSound_Cue" _returnvalue "0, 0, 0" 1.0 1.0 0.0 0 0 0 0)
      (Timeline|OpenDoorTimeline ReverseFromEnd))))

(fn ConstructionScript)