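; Level transition tool actor that teleports the player pawn when a first-transition event fires.
; On BeginPlay it binds its handler to that event.
; The handler shifts player 0's pawn by the position delta from FromActor to ToActor and adds their rotation delta to the pawn's rotation.
; The pawn's world-space offset from the reference actor is preserved without being rotated.
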(event Custom|FirstTransition_Event
  (bind _returnvalue (Game|Player|GetPlayerPawn 0))
  (bind _toactor (Variables|Default|GetToActor))
  (bind _fromactor (Variables|Default|GetFromActor))
  (Transformation|SetActorLocationAndRotation _returnvalue (+ (Transformation|GetActorLocation _returnvalue) (- (Transformation|GetActorLocation _toactor) (Transformation|GetActorLocation _fromactor))) (Math|Rotator|CombineRotators (Transformation|GetActorRotation _returnvalue) (Math|Rotator|Delta(Rotator) (Transformation|GetActorRotation _toactor) (Transformation|GetActorRotation _fromactor)))))

(event EventBeginPlay
  (EventDispatchers|BindEventtoFirstTransition (delegate Custom|FirstTransition_Event)))

(fn ConstructionScript)